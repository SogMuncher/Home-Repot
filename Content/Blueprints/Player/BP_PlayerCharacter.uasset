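; Player character Blueprint that provides basic movement, look and jump from input events.
; Forward and right input feed AddMovementInput along vectors taken from the full control rotation, with pitch not stripped out.
; Look and turn input drive controller pitch and yaw directly, and the jump event calls Jump.
; BeginPlay and the construction script are empty.
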(event Custom|Character_MoveForward
  (params (Triggered :type Float%20%28double-precision%29))
  (Pawn|Input|AddMovementInput (Math|Vector|GetForwardVector (Pawn|GetControlRotation :!class /Script/Engine.Pawn)) Triggered false))

(event Custom|Character_MoveRight
  (params (Triggered :type Float%20%28double-precision%29))
  (Pawn|Input|AddMovementInput (Math|Vector|GetRightVector (Pawn|GetControlRotation :!class /Script/Engine.Pawn)) Triggered false))

(event Custom|Character_LookUp
  (params (Triggered :type Float%20%28double-precision%29))
  (Pawn|Input|AddControllerPitchInput Triggered))

(event Custom|Character_Turn
  (params (Triggered :type Float%20%28double-precision%29))
  (Pawn|Input|AddControllerYawInput Triggered))

(event Custom|Character_Jump
  (params (Triggered :type Float%20%28double-precision%29))
  (Character|Jump))

(event EventBeginPlay)

(fn ConstructionScript)