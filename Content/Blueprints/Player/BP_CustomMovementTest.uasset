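; Test pawn for a custom movement component, with a capsule, spring arm and camera.
; Each tick it prints the normalized last valid movement input vector as debug text.
; Disconnected experiments remain in the graph: mapping capsule speed to spring arm length using ground or air max speed, and setting camera roll from the capsule's roll.
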(event EventBeginPlay)

(event EventTick
  (params (DeltaSeconds :type Float%20%28single-precision%29))
  (Development|PrintText (Utilities|Text|ToText(String) (Math|Vector|Normalize (Variables|/Script/GD73MegaJam2025.CustomPawnMovementComponent|GetLastValidMovementInputVector (Variables|Default|GetCustomPawnMovement))))))

(fn ConstructionScript)